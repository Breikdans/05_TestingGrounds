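; AI controller for NPCs that starts the Patrol behavior tree on the PatrolData blackboard at BeginPlay.
; AI perception updates only print a debug string with the controlled pawn, sense class and perceived actor.
; FindPatrolRoute casts the pawn to PatrollingGuard and writes the first element of an array built from that guard into the Waypoint blackboard key.
; Nothing in this graph calls FindPatrolRoute.
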(event `self.ReceiveBeginPlay`
  (`self.UseBlackboard` "/Game/NPC/AI/PatrolData.PatrolData")
  (`self.RunBehaviorTree` "/Game/NPC/AI/Patrol.Patrol"))

(event `self.AIPerception.OnTargetPerceptionUpdated`
  (params (Actor :type "Actor Object Reference") (Stimulus :type "AIStimulus Structure"))
  (bind _returnvalue (`AIPerceptionSystem.GetSenseClassForStimulus` Stimulus))
  (`KismetSystemLibrary.PrintString` (`KismetStringLibrary.Concat_StrStr` (`KismetSystemLibrary.GetObjectName` (`self.K2_GetPawn`)) " " (`KismetSystemLibrary.GetClassDisplayName` _returnvalue) " " (`KismetSystemLibrary.GetDisplayName` Actor))))

(fn `Find Patrol Route`
  (params (Blackboard :type "BlackboardComponent Object Reference"))
  (bind _aspatrolling_guard (cast `/Game/NPC/Character/PatrollingGuard` (`self.K2_GetPawn`)))
  (`BlackboardComponent.SetValueAsObject` Blackboard "Waypoint" (`|GetArrayItem` (`|MakeArray` _aspatrolling_guard :!type "Actor Object Reference"))))

(fn `UserConstructionScript`)